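; Player character for the water boat sections, driven by physics forces on a Cube component with Enhanced Input.
; BeginPlay adds the water mapping context and gives one push along the Cube's right vector, its travel axis.
; Steering adds sideways acceleration along the forward vector, while forward/backward input is labelled disabled.
; Interact, gated by CanLoadStage, stops physics, plays a reversed fade and opens LevelToLoad after a delay.
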(event Input|EnhancedActionEvents|EnhancedInputActionIA_BoatMove
  (params (ActionValue :type Float%20%28double-precision%29) (ElapsedSeconds :type Float%20%28double-precision%29) (TriggeredSeconds :type Float%20%28double-precision%29) (InputAction :type Input%20Action%20Object%20Reference :default "/Game/Water/Input/Actions/IA_BoatMove.IA_BoatMove"))
  ;[1 1 1] Boat Forward/Backward [Disabled]
  (Physics|AddForce (Variables|Default|GetCube) (* (Math|Vector|RotateVector (Math|Vector|MakeVector 0.0 (/ ActionValue 3e+02) 0.0) (Transformation|GetWorldRotation (Variables|Default|GetCube))) (Variables|Default|GetConstantBoatSpeed)) "None" true))

(event Input|EnhancedActionEvents|EnhancedInputActionIA_BoatSteer
  (params (ActionValue :type Float%20%28double-precision%29) (ElapsedSeconds :type Float%20%28double-precision%29) (TriggeredSeconds :type Float%20%28double-precision%29) (InputAction :type Input%20Action%20Object%20Reference :default "/Game/Water/Input/Actions/IA_BoatSteer.IA_BoatSteer"))
  (bind _cube (Variables|Default|GetCube))
  ;[1 1 1] Boat Sideways Movement
  (Physics|AddForce _cube (* (* ActionValue -6e+02) (Math|Vector|GetForwardVector _cube)) "None" true))

(event Input|EnhancedActionEvents|EnhancedInputActionIA_BoatInteract
  (params (ActionValue :type Boolean) (ElapsedSeconds :type Float%20%28double-precision%29) (TriggeredSeconds :type Float%20%28double-precision%29) (InputAction :type Input%20Action%20Object%20Reference :default "/Game/Water/Input/Actions/IA_BoatInteract.IA_BoatInteract"))
  ;[1 1 1] Getting into Boat
  (if (Variables|Default|GetCanLoadStage)
    (Variables|Default|SetCanLoadStage false)
    (Physics|SetSimulatePhysics (Variables|Default|GetCube) false)
    (bind _returnvalue (UserInterface|CreateWidget "/Game/GUI/Fade.Fade_C"))
    (UserInterface|Viewport|AddtoViewport _returnvalue 0)
    (Class|UserWidget|PlayAnimationReverse _returnvalue (Variables|/Game/GUI/Fade.Fade_C|GetFadeInOut _returnvalue) 1.0 false)
    (Utilities|FlowControl|Delay 3.0)
    (Game|OpenLevel(byObjectReference) (Variables|Default|GetLevelToLoad))))

(event EventBeginPlay
  ;[0.1562 1 0] BeginPlay
  (bind _asplayer_controller (Utilities|Casting|CastToPlayerController (Pawn|GetController)))
  (Utilities|IsValid (PlayerController|LocalPlayerSubsystems|GetEnhancedInputLocalPlayerSubsystem _asplayer_controller)
    (:Is%20Valid
      (Input|AddMappingContext (PlayerController|LocalPlayerSubsystems|GetEnhancedInputLocalPlayerSubsystem _asplayer_controller) "/Game/Water/Input/IMC_Water.IMC_Water" 0 "(bIgnoreAllPressedKeysUntilRelease=True,bForceImmediately=False,bNotifyUserSettings=False)")
      (Physics|AddForce (Variables|Default|GetCube) (* (Variables|Default|GetConstantBoatSpeed) (Math|Vector|GetRightVector (Variables|Default|GetCube))) "None" false))))

(event Input|KeyboardEvents|S
  (params (Key :type Key%20Structure :default "None")))

(fn ConstructionScript)