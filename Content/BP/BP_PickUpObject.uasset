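; BP_PickUpObject is an object with a static mesh, trigger and glow that can be flagged as pick-up-able.
; The PickUp event sets IsPickUpable and shows the Glow component.
; Trigger overlaps check the third-person character's CanPickup, but their glow visibility calls are disabled.
; EnablePhysics and DisablePhysics events exist for toggling mesh simulation, but their SetSimulatePhysics calls are also disabled.
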(event OnComponentBeginOverlap(Trigger)
  (params (OverlappedComponent :type Primitive%20Component%20Object%20Reference) (OtherActor :type Actor%20Object%20Reference) (OtherComp :type Primitive%20Component%20Object%20Reference) (OtherBodyIndex :type Integer) (bFromSweep :type Boolean) (SweepResult :type Hit%20Result%20Structure%20%28by%20ref%29))
  ;[1 1 1] Toggle Prompt Message Visibility
  (bind _asbp_third_person_character (Utilities|Casting|CastToBP_ThirdPersonCharacter OtherActor))
  (if (Variables|/Game/ThirdPerson/Blueprints/BP_ThirdPersonCharacter.BP_ThirdPersonCharacter_C|GetCan%20Pickup _asbp_third_person_character)
    (Rendering|SetVisibility (Variables|Default|GetGlow) (Variables|/Game/ThirdPerson/Blueprints/BP_ThirdPersonCharacter.BP_ThirdPersonCharacter_C|GetCan%20Pickup _asbp_third_person_character) false)))

(event OnComponentEndOverlap(Trigger)
  (params (OverlappedComponent :type Primitive%20Component%20Object%20Reference) (OtherActor :type Actor%20Object%20Reference) (OtherComp :type Primitive%20Component%20Object%20Reference) (OtherBodyIndex :type Integer))
  ;[1 1 1] Toggle Prompt Message Visibility
  (bind _asbp_third_person_character (Utilities|Casting|CastToBP_ThirdPersonCharacter OtherActor))
  (if (not (Variables|/Game/ThirdPerson/Blueprints/BP_ThirdPersonCharacter.BP_ThirdPersonCharacter_C|GetCan%20Pickup _asbp_third_person_character))
    (Rendering|SetVisibility (Variables|Default|GetGlow) (Variables|/Game/ThirdPerson/Blueprints/BP_ThirdPersonCharacter.BP_ThirdPersonCharacter_C|GetCan%20Pickup _asbp_third_person_character) false)))

(event Custom|EnablePhysics
  ;[1 1 1] Call Enable/Disable Physics
  (Physics|SetSimulatePhysics (Variables|Default|GetStaticMesh) true))

(event Custom|DisablePhysics
  ;[1 1 1] Call Enable/Disable Physics
  (Physics|SetSimulatePhysics (Variables|Default|GetStaticMesh) false))

(event Custom|PickUp
  ;[1 1 1] Set Object as Pick-Up-able
  (bind _output_get (Variables|Default|SetIsPickUpable true))
  (Rendering|SetVisibility (Variables|Default|GetGlow) _output_get false))

(fn ConstructionScript)