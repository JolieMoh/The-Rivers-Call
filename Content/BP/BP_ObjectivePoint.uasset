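; BP_ObjectivePoint is a trigger volume that shows a quest objective on screen when the player first enters it.
; It creates a W_ObjectiveMenu widget at BeginPlay, then on overlap fills in the title and content, animates it in and flags the objective in progress.
; ObjectiveCompleted plays completion animations and clears that flag before testing it, so the delayed fade-out never runs.
; The construction script sizes the box from ObjectiveBoxSize.
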(event OnComponentBeginOverlap(ObjectiveBox)
  (params (OverlappedComponent :type Primitive%20Component%20Object%20Reference) (OtherActor :type Actor%20Object%20Reference) (OtherComp :type Primitive%20Component%20Object%20Reference) (OtherBodyIndex :type Integer) (bFromSweep :type Boolean) (SweepResult :type Hit%20Result%20Structure%20%28by%20ref%29))
  (bind _w_objectivemenu (Variables|Default|GetW_ObjectiveMenu))
  (if (== OtherActor (Game|GetPlayerCharacter 0))
    (Utilities|FlowControl|DoOnce false
      (:Completed
        (Variables|/Game/GUI/W_ObjectiveMenu.W_ObjectiveMenu_C|SetObjectiveTitle%20Text _w_objectivemenu (Variables|Default|GetObjectiveTitle%20Text))
        (Variables|/Game/GUI/W_ObjectiveMenu.W_ObjectiveMenu_C|SetObjectiveContent%20Text _w_objectivemenu (Variables|Default|GetObjectiveContent%20Text))
        (UserInterface|Viewport|AddtoViewport _w_objectivemenu 0)
        (UserInterface|Animation|PlayAnimation _w_objectivemenu (Variables|/Game/GUI/W_ObjectiveMenu.W_ObjectiveMenu_C|GetFadeOutMenu _w_objectivemenu) 0.0 1 "Reverse" 1.0 false)
        (UserInterface|Animation|PlayAnimation _w_objectivemenu (Variables|/Game/GUI/W_ObjectiveMenu.W_ObjectiveMenu_C|GetNewObjective _w_objectivemenu) 0.0 1 "Forward" 1.0 false)
        (Variables|Default|SetObjectiveInProgress? true)))))

(event Custom|ObjectiveCompleted
  (bind _w_objectivemenu (Variables|Default|GetW_ObjectiveMenu))
  (bind _w_objectivemenu_2 (Variables|Default|GetW_ObjectiveMenu))
  (UserInterface|Animation|PlayAnimation _w_objectivemenu_2 (Variables|/Game/GUI/W_ObjectiveMenu.W_ObjectiveMenu_C|GetObjectiveContentComplete _w_objectivemenu_2) 0.0 1 "Forward" 1.0 false)
  (UserInterface|Animation|PlayAnimation _w_objectivemenu_2 (Variables|/Game/GUI/W_ObjectiveMenu.W_ObjectiveMenu_C|GetObjectiveTitleComplete _w_objectivemenu_2) 0.0 1 "Forward" 1.0 false)
  (bind _output_get (Variables|Default|SetObjectiveInProgress? false))
  (if _output_get
    (Utilities|FlowControl|Delay 5.0)
    (UserInterface|Animation|PlayAnimation _w_objectivemenu (Variables|/Game/GUI/W_ObjectiveMenu.W_ObjectiveMenu_C|GetFadeOutMenu _w_objectivemenu) 0.0 1 "Forward" 1.0 false)))

(event EventBeginPlay
  (bind _returnvalue (UserInterface|CreateWidget "/Game/GUI/W_ObjectiveMenu.W_ObjectiveMenu_C" 0 (Variables|Default|GetObjectiveTitle%20Text) (Variables|Default|GetObjectiveContent%20Text)))
  (Variables|Default|SetW_ObjectiveMenu _returnvalue))

(fn ConstructionScript
  (Components|Box|SetBoxExtent (Variables|Default|GetObjectiveBox) (Variables|Default|GetObjective%20Box%20Size) true))