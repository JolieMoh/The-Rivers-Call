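; BP_spring is a spring pad actor that launches the third-person player character upward when it hits the pad's Cube.
; The Cube's hit event checks that the other actor is a BP_ThirdPersonCharacter, then plays pickup and jump sounds in 2D.
; It calls Jump and overrides the movement component's vertical velocity with a strong fixed boost, keeping horizontal velocity, then prints a debug string.
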(event OnComponentHit(Cube)
  (params (HitComponent :type Primitive%20Component%20Object%20Reference) (OtherActor :type Actor%20Object%20Reference) (OtherComp :type Primitive%20Component%20Object%20Reference) (NormalImpulse :type Vector :default "0, 0, 0") (Hit :type Hit%20Result%20Structure%20%28by%20ref%29))
  (if (Utilities|ClassIsChildOf (Utilities|GetClass OtherActor) "/Game/ThirdPerson/Blueprints/BP_ThirdPersonCharacter.BP_ThirdPersonCharacter_C")
    (Audio|PlaySound2D "/Engine/VREditor/Sounds/UI/Object_PickUp.Object_PickUp" 1.0 1.0 0.0 0 0)
    (Audio|PlaySound2D "/Game/SFX/jump2.jump2" 1.0 1.0 0.0 0 0)
    (bind _asbp_third_person_character (Utilities|Casting|CastToBP_ThirdPersonCharacter OtherActor))
    (Character|Jump _asbp_third_person_character)
    (Variables|/Script/Engine.MovementComponent|SetVelocity (Pawn|GetMovementComponent _asbp_third_person_character) (Math|Vector|MakeVector (.x (Variables|/Script/Engine.MovementComponent|GetVelocity (Pawn|GetMovementComponent _asbp_third_person_character))) (.y (Variables|/Script/Engine.MovementComponent|GetVelocity (Pawn|GetMovementComponent _asbp_third_person_character))) 3e+03))
    (Development|PrintString "Hello")))

(event EventBeginPlay)

(event Collision|EventActorBeginOverlap
  (params (OtherActor :type Actor%20Object%20Reference)))

(event EventTick
  (params (DeltaSeconds :type Float%20%28single-precision%29)))

(fn ConstructionScript)